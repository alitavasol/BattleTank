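; Player-controllable tank Blueprint that wires components and input for driving, camera orbit and firing.
; On BeginPlay it passes barrel and turret to the aiming component, and both tracks to the movement component.
; Movement axes feed the movement component, with opposite directions sharing one function, while the fire action calls the aiming component.
; Camera yaw and pitch rotate separate components locally, scaled by delta time for frame-rate independence.
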(event `self.ReceiveBeginPlay`
  (`TankAimingComponent.Initialize` (`self.TankAimingComp`) (`self.TankBarrel`) (`self.TankTurret`))
  (`TankNavMovementComponent.Initialize` (`self.TankNavMovement`) (`self.RightTrack`) (`self.LeftTrack`)))

(event `InputAxis|MoveForward`
  (params (AxisValue :type "Float (single-precision)"))
  ;[1 1 1] Movement Input Setup.
  (`TankNavMovementComponent.IntendMoveForward` (`self.TankNavMovement`) AxisValue))

(event `InputAxis|Camera Moving in Z(Yaw)`
  (params (AxisValue :type "Float (single-precision)"))
  ;[1 1 1] Camera Movement in Z (Yaw)
  (`SceneComponent.K2_AddLocalRotation` (`self.Camera Z Rotator`) (`KismetMathLibrary.MakeRotator` 0.0 0.0 (* AxisValue (`GameplayStatics.GetWorldDeltaSeconds`) 100.0)) false false))

(event `InputAxis|MoveBackward`
  (params (AxisValue :type "Float (single-precision)"))
  ;[1 1 1] Movement Input Setup.
  (`TankNavMovementComponent.IntendMoveForward` (`self.TankNavMovement`) AxisValue))

(event `InputAxis|TurnRight`
  (params (AxisValue :type "Float (single-precision)"))
  ;[1 1 1] Movement Input Setup.
  (`TankNavMovementComponent.TurnRight` (`self.TankNavMovement`) AxisValue))

(event `InputAxis|Camera Moving in Y(Pich)`
  (params (AxisValue :type "Float (single-precision)"))
  ;[1 1 1] Camera Movement in Y (Pich)
  (`SceneComponent.K2_AddLocalRotation` (`self.SpringArm(Y Rotator)`) (`KismetMathLibrary.MakeRotator` 0.0 (* AxisValue (`GameplayStatics.GetWorldDeltaSeconds`) 100.0)) false false))

(event `InputAxis|TurnLeft`
  (params (AxisValue :type "Float (single-precision)"))
  ;[1 1 1] Movement Input Setup.
  (`TankNavMovementComponent.TurnRight` (`self.TankNavMovement`) AxisValue))

(event `InputAction|Fire Projectile`
  (params (Key :type "Key Structure"))
  ;[1 1 1] Fire Projectile Input Setup.
  (:`Pressed`
    (`TankAimingComponent.Fire` (`self.TankAimingComp`))))

(fn `UserConstructionScript`)